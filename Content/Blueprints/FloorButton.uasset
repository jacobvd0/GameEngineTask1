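; FloorButton is a pressure-plate actor that opens a linked Door when something overlaps its Hitbox.
; Each Hitbox begin overlap increments an item count, turns the Trigger material red and calls BothDoorsOpen on DoorToActivate.
; End overlaps passing a TestCube or Pawn class cast decrement the count, reopening the door while items remain or turning the Trigger green otherwise.
; Nothing here closes the door.
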(event `self.Hitbox.OnComponentBeginOverlap`
  (params (OverlappedComponent :type "PrimitiveComponent Object Reference") (OtherActor :type "Actor Object Reference") (OtherComp :type "PrimitiveComponent Object Reference") (OtherBodyIndex :type Integer) (bFromSweep :type Boolean) (SweepResult :type "HitResult Structure (by ref)"))
  (if (`GameplayStatics.ObjectIsA` OverlappedComponent (`GameplayStatics.GetObjectClass` (`self.Hitbox`)))
    (set `self.ItemsInHitbox` (+ 1 (`self.ItemsInHitbox`)))
    (`PrimitiveComponent.SetMaterial` (`self.Trigger`) 0 "/Game/Materials/Red.Red")
    (bind _asdoor (cast `/Game/Blueprints/Door` (`self.DoorToActivate`) :!label _label))
    (`/Game/Blueprints/Door.Both Doors Open` _asdoor)))

(event `self.ReceiveActorEndOverlap`
  (params (OtherActor :type "Actor Object Reference"))
  (bind _returnvalue (`GameplayStatics.GetObjectClass` OtherActor))
  (bind _trigger (`self.Trigger`))
  (castclass `/Game/Blueprints/TestCube` _returnvalue
    (:`then`
      _)
    (:`CastFailed`
      (castclass `Pawn` _returnvalue)))
  (bind _output_get (set `self.ItemsInHitbox` (- (`self.ItemsInHitbox`) 1)))
  (if (> _output_get 0)
    (`PrimitiveComponent.SetMaterial` _trigger 0 "/Game/Materials/Red.Red")
    (goto _label)
    (else
      (`PrimitiveComponent.SetMaterial` _trigger 0 "/Game/Materials/Green.Green"))))

(event `OnActorEndOverlap_Event`
  (params (OverlappedActor :type "Actor Object Reference") (OtherActor :type "Actor Object Reference")))

(fn `UserConstructionScript`)