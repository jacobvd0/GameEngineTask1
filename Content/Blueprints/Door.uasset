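; Door Blueprint for a two-panel sliding door, opened and closed through custom events.
; BothDoorsOpen checks that DoorID is 0, then runs two timelines that slide DoorLeft and DoorRight along local X at a fixed height.
; OpenDoor and closedoor drive only the right panel through the Goback timeline.
; Closing reverses the timelines and, unlike BothDoorsOpen, does not check DoorID.
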(event `Both Doors Open`
  (if (== (`self.Door ID`) 0)
    (`self.OpenDoor`)
    (bind (_direction _newtrack_0) (`Timeline|Door Open` :!label _label)
      (:`Update`
        (`SceneComponent.K2_SetRelativeLocation` (`self.DoorLeft`) (`KismetMathLibrary.MakeVector` _newtrack_0 0.0 120.0) false false)))))

(event `Both Doors Close`
  (`self.close door`)
  (goto _label :!via `Reverse`))

(event `OpenDoor`
  (bind (_direction _newtrack_0) (`Timeline|goback` :!label _label_2)
    (:`Update`
      (`SceneComponent.K2_SetRelativeLocation` (`self.DoorRight`) (`KismetMathLibrary.MakeVector` _newtrack_0 0.0 120.0) false false))))

(event `close door`
  (goto _label_2 :!via `Reverse`))

(fn `UserConstructionScript`)