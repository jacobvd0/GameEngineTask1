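; Level manager that shows the level number, hint text and a running game timer on the in-game HUD.
; BeginPlay writes LevelNumber and HintText into the IngameHUD widget, reached through player controller 0's PlayerHUD.
; Tick repeats that lookup, splits game time into zero-padded MM:SS, builds TimerText through a custom Append event and pushes it to the timer.
; Failed casts only print a message.
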(event `self.ReceiveBeginPlay`
  (bind _asplayer_controller (cast `PlayerController` (`GameplayStatics.GetPlayerController` 0))
    (:`then`
      (bind _asplayer_hud (cast `/Game/Widgets/PlayerHUD` (`PlayerController.GetHUD` _asplayer_controller))
        (:`then`
          (bind _ingamehud (`/Game/Widgets/PlayerHUD.IngameHUD` _asplayer_hud))
          (set `TextBlock.Text` (`KismetTextLibrary.Conv_StringToText` (`KismetStringLibrary.Concat_StrStr` "Level " (`KismetStringLibrary.Conv_IntToString` (`self.LevelNumber`)))) (`/Game/Widgets/IngameHUD.CurrentLevel` _ingamehud))
          (set `TextBlock.Text` (`self.HintText`) (`/Game/Widgets/IngameHUD.LevelHint` _ingamehud)))
        (:`CastFailed`
          (`KismetSystemLibrary.PrintText` "Failed to cast to PlayerHUD"))))
    (:`CastFailed`
      (`KismetSystemLibrary.PrintText` "Failed to cast to player controller"))))

(event `self.ReceiveTick`
  (params (DeltaSeconds :type "Float (single-precision)"))
  (bind _returnvalue (`KismetSystemLibrary.GetGameTimeInSeconds`))
  (bind _asplayer_controller (cast `PlayerController` (`GameplayStatics.GetPlayerController` 0))
    (:`then`
      (bind _asplayer_hud (cast `/Game/Widgets/PlayerHUD` (`PlayerController.GetHUD` _asplayer_controller))
        (:`then`
          (bind _output_get (set `self.minutes` (`KismetMathLibrary.FTrunc` (`KismetMathLibrary.SafeDivide` _returnvalue 60.0))))
          (set `self.seconds` (`KismetMathLibrary.FTrunc` (- _returnvalue (* _output_get 60))))
          (if (< (`self.minutes`) 10)
            (if (< (`self.seconds`) 10)
              (`self.Append` "0" (`KismetTextLibrary.Conv_IntToText` (`self.minutes`)) ":" "0" (`KismetTextLibrary.Conv_IntToText` (`self.seconds`)))
              (else
                (`self.Append` "0" (`KismetTextLibrary.Conv_IntToText` (`self.minutes`)) ":" (`KismetTextLibrary.Conv_IntToText` (`self.seconds`)))))
            (elif (< (`self.seconds`) 10)
              (`self.Append` (`KismetTextLibrary.Conv_IntToText` (`self.minutes`)) ":" "0" (`KismetTextLibrary.Conv_IntToText` (`self.seconds`)))
              (else
                (`self.Append` (`KismetTextLibrary.Conv_IntToText` (`self.minutes`)) ":" (`KismetTextLibrary.Conv_IntToText` (`self.seconds`))))))
          (set `TextBlock.Text` (`self.TimerText`) (`/Game/Widgets/IngameHUD.GameTimer` (`/Game/Widgets/PlayerHUD.IngameHUD` _asplayer_hud))))
        (:`CastFailed`
          (`KismetSystemLibrary.PrintText` "Failed to cast to PlayerHUD"))))
    (:`CastFailed`
      (`KismetSystemLibrary.PrintText` "Failed to cast to player controller"))))

(event `Append`
  (params (A :type Text) (B :type Text) (C :type Text) (D :type Text) (E :type Text))
  (set `self.TimerText` (`KismetTextLibrary.Conv_StringToText` (`KismetStringLibrary.Concat_StrStr` (`KismetTextLibrary.Conv_TextToString` A) (`KismetTextLibrary.Conv_TextToString` B) (`KismetTextLibrary.Conv_TextToString` C) (`KismetTextLibrary.Conv_TextToString` D) (`KismetTextLibrary.Conv_TextToString` E)))))

(fn `UserConstructionScript`)